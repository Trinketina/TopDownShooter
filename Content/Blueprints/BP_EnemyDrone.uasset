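; BP_EnemyDrone is an enemy that deals repeated contact damage to the player and counts as a kill when it dies.
; A looping timer starts when the player overlaps it, applies damage through the player's AffectHealth, and is cleared when the overlap ends.
; Its own AffectHealth event runs CalculateHealth, and on death destroys the drone and increments the kill count on the BP_TDSMode UI.
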(event Custom|DamagePlayer
  ;[1 1 1] Damage
  (Default|AffectHealth (Variables|Default|GetPlayer) (Variables|Default|GetDamageDelta)))

(event EventAffectHealth
  (params (Delta :type Float%20%28single-precision%29))
  ;[1 1 1] interface
  (Class|TDSCharacter|CalculateHealth Delta)
  (if (Variables|Default|GetisDead)
    (Actor|DestroyActor)
    (bind _asbp_tdsmode (Utilities|Casting|CastToBP_TDSMode (Game|GetGameMode)))
    (Default|IncrementKillCount (Variables|/Game/Blueprints/BP_TDSMode.BP_TDSMode_C|GetUI _asbp_tdsmode))))

(event Collision|EventActorBeginOverlap
  (params (OtherActor :type Actor%20Object%20Reference))
  ;[1 1 1] Damage
  (bind _asbp_player (Utilities|Casting|CastToBP_Player OtherActor))
  (Variables|Default|SetPlayer _asbp_player)
  (Utilities|Time|SetTimerbyFunctionName 0 "DamagePlayer" 0.5 true))

(event Collision|EventActorEndOverlap
  (params (OtherActor :type Actor%20Object%20Reference))
  ;[1 1 1] Damage
  (if (== OtherActor (Variables|Default|GetPlayer))
    (Utilities|Time|ClearTimerbyFunctionName 0 "DamagePlayer")))

(fn ConstructionScript)