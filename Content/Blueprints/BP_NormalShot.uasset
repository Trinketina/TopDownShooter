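; BP_NormalShot is a shot actor that damages what it overlaps, sparing actors tagged Player.
; On overlap with an untagged actor implementing I_Damage, it sends AffectHealthMessage with its DamageDelta and destroys itself.
; Tick accumulates a Lifespan counter and destroys the shot after five seconds.
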(event Collision|EventActorBeginOverlap
  (params (OtherActor :type Actor%20Object%20Reference))
  (if (Utilities|DoesObjectImplementInterface OtherActor "/Game/Blueprints/I_Damage.I_Damage_C")
    (if (not (Actor|ActorHasTag OtherActor "Player"))
      (Class|IDamage|AffectHealth(Message) OtherActor (Variables|Default|GetDamageDelta))
      (Actor|DestroyActor))))

(event EventTick
  (params (DeltaSeconds :type Float%20%28single-precision%29))
  (bind _output_get (Variables|Default|SetLifespan (+ DeltaSeconds (Variables|Default|GetLifespan))))
  (if (>= _output_get 5.0)
    (Actor|DestroyActor)))

(fn ConstructionScript)