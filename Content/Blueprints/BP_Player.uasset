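; Player pawn for a top-down shooter that moves on world axes and fires BP_NormalShot from BulletSpawn.
; Holding Shoot repeats fire through a Delay loop.
; Mouse movement direction, rather than cursor position, sets aim: velocity above a deadzone smoothly interpolates control yaw each tick.
; BeginPlay registers the spawn transform with BP_TDSMode; on death, AffectHealth disables input, then after a pause requests respawn and destroys the actor.
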(event Custom|FireBasicShot
  ;[1 1 1] Fire Weapon
  (if (Variables|Default|GetcanShoot)
    (Game|SpawnActorfromClass "/Game/Blueprints/BP_NormalShot.BP_NormalShot_C" (Transformation|GetWorldTransform (Variables|Default|GetBulletSpawn)) "Undefined" 0 0)))

(event EventAffectHealth
  (params (Delta :type Float%20%28single-precision%29))
  ;[1 1 1] interface
  (Class|TDSCharacter|CalculateHealth Delta)
  (if (Variables|Default|GetisDead)
    (Input|DisableInput 0)
    (Utilities|FlowControl|Delay 1.0)
    (Default|RespawnPlayer (Variables|Default|GetGameMode))
    (Actor|DestroyActor)))

(event EventTick
  (params (DeltaSeconds :type Float%20%28single-precision%29))
  (bind _mouseinput (CallFunction|GetMouseVelocity))
  (bind _returnvalue (Game|GetPlayerController 0))
  ;[1 1 1] PlayerRotation
  (if (CallFunction|GetMouseDeadzone)
    (Pawn|SetControlRotation _returnvalue (Math|Interpolation|RInterpTo (Pawn|GetControlRotation _returnvalue :!class /Script/Engine.Controller) (Math|Rotator|MakeRotator 0.0 0.0 (Class|KismetMathLibrary|DegAtan2 (.x _mouseinput) (.y _mouseinput))) (Utilities|Time|GetWorldDeltaSeconds) 7.0))))

(event EventBeginPlay
  ;[1 1 1] init
  (bind _asbp_tdsmode (Utilities|Casting|CastToBP_TDSMode (Game|GetGameMode)))
  (bind _output_get (Variables|Default|SetGameMode _asbp_tdsmode))
  (Variables|/Game/Blueprints/BP_TDSMode.BP_TDSMode_C|SetSpawnpoint _output_get (Transformation|GetActorTransform)))

(event Input|ActionEvents|InputActionShoot
  (params (Key :type Key%20Structure :default "None"))
  ;[1 1 1] Fire Weapon
  (:Pressed
    (bind _output_get (Variables|Default|SetcanShoot true))
    (if _output_get :!label _label
      (CallFunction|FireBasicShot)
      (Utilities|FlowControl|Delay 0.2)
      (goto _label)))
  (:Released
    (Variables|Default|SetcanShoot false)))

(event Input|AxisEvents|InputAxisMoveForward
  (params (AxisValue :type Float%20%28single-precision%29))
  ;[1 1 1] movement
  (Pawn|Input|AddMovementInput "1.000000, 0, 0" AxisValue false))

(event Input|AxisEvents|InputAxisMoveHorizontal
  (params (AxisValue :type Float%20%28single-precision%29))
  ;[1 1 1] movement
  (Pawn|Input|AddMovementInput "0.000000,1.000000, 0" AxisValue false))

(fn ConstructionScript)

(fn GetMouseVelocity
  (bind _returnvalue (Game|GetPlayerController 0))
  (bind (_deltax _deltay) (Class|PlayerController|GetInputMouseDelta _returnvalue))
  (return (/ (Math|Vector2D|MakeVector2D _deltax _deltay) (Utilities|Time|GetWorldDeltaSeconds))))

(fn GetMouseDeadzone
  (return (> (Math|Vector2D|Vector2DLength (CallFunction|GetMouseVelocity)) (Variables|Default|GetmouseDeadzone))))