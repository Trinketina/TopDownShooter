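; BP_TDSMode is the game mode that starts enemy and power-up spawning, shows the HUD and handles player respawn.
; On BeginPlay it takes the first BP_Spawner in the level and sets looping name-based timers on its SpawnEnemy and SpawnPowerUp functions, then adds a UI_HUD widget to the viewport.
; RespawnPlayer spawns a new BP_Player at the stored spawn transform and has player controller 0 possess it.
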(event Custom|RespawnPlayer
  ;[1 1 1] Respawn
  (bind _returnvalue (Game|SpawnActorfromClass "/Game/Blueprints/BP_Player.BP_Player_C" (Variables|Default|GetSpawnpoint) "Undefined" 0 0))
  (Pawn|Possess (Game|GetPlayerController 0) _returnvalue))

(event EventBeginPlay
  (bind _outactors (Actor|GetAllActorsOfClass "/Game/Blueprints/BP_Spawner.BP_Spawner_C"))
  (bind _output_get (Variables|Default|SetSpawner (Utilities|Array|Get(acopy) _outactors)))
  (Utilities|Time|SetTimerbyFunctionName _output_get "SpawnEnemy" (Variables|Default|GetSpawnTime) true)
  (Utilities|Time|SetTimerbyFunctionName _output_get "SpawnPowerUp" (Variables|Default|GetPowerupSpawnTime) true)
  (bind _returnvalue (UserInterface|CreateWidget "/Game/Blueprints/UI_HUD.UI_HUD_C"))
  (bind _output_get_2 (Variables|Default|SetUI _returnvalue))
  (UserInterface|Viewport|AddtoViewport _output_get_2 0))

(fn ConstructionScript)