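; Spawner actor that places enemy drones and power-ups at random points inside its SpawnVolume box.
; SpawnEnemy and SpawnPowerUp each count live actors of their class and spawn only below MaxEnemies or MaxPowerups.
; Enemies spawn as AI pawns, while each power-up is a coin flip between the Attack and Speed variants.
; Both are custom events with no trigger or timer in this graph.
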(event Custom|SpawnEnemy
  (bind _spawnvolume (Variables|Default|GetSpawnVolume))
  ;[1 1 1] Spawn Enemy
  (bind _outactors (Actor|GetAllActorsOfClass "/Game/Blueprints/BP_EnemyDrone.BP_EnemyDrone_C"))
  (if (< (Utilities|Array|Length _outactors) (Variables|Default|GetMaxEnemies))
    (AI|SpawnAIFromClass "/Game/Blueprints/BP_EnemyDrone.BP_EnemyDrone_C" 0 (Math|Random|RandomPointinBoundingBox (Transformation|GetWorldLocation _spawnvolume) (Components|Box|GetScaledBoxExtent _spawnvolume)) "0, 0, 0" false 0)))

(event Custom|SpawnPowerUp
  (bind _spawnvolume (Variables|Default|GetSpawnVolume))
  (bind _returnvalue (Transformation|GetWorldLocation _spawnvolume))
  (bind _returnvalue_2 (Components|Box|GetScaledBoxExtent _spawnvolume))
  (bind _returnvalue_3 (Math|Random|RandomPointinBoundingBox _returnvalue _returnvalue_2))
  (bind _returnvalue_4 (Math|Conversions|ToTransform(Vector) _returnvalue_3))
  ;[1 1 1] Spawn Powerups
  (bind _outactors (Actor|GetAllActorsOfClass "/Game/Blueprints/BP_PowerUp.BP_PowerUp_C"))
  (if (< (Utilities|Array|Length _outactors) (Variables|Default|GetMaxPowerups))
    (if (Math|Random|RandomBool)
      (Game|SpawnActorfromClass "/Game/Blueprints/BP_PowerUp_Attack.BP_PowerUp_Attack_C" _returnvalue_4 "Undefined" 0 0)
      (else
        (Game|SpawnActorfromClass "/Game/Blueprints/BP_PowerUp_Speed.BP_PowerUp_Speed_C" _returnvalue_4 "Undefined" 0 0)))))

(fn ConstructionScript)